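; BP_Menu3DActor is a 3D menu station actor that shows a menu widget and moves the player's view between linked menus.
; On BeginPlay it binds to the transition event of its F_WBP_Menu3D widget and disables its own collision.
; A transition event picks a valid entry from LinkedMenus, swaps collision to that menu, and blends the player camera to it with an eased view target blend.
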(event `self.ReceiveBeginPlay`
  (bind _asf_wbp_menu_3d (cast `/Game/Menu/Widgets/F_WBP_Menu3D` (`WidgetComponent.GetUserWidgetObject` (`self.Widget`))))
  (add `/Game/Menu/Widgets/F_WBP_Menu3D.TransitionMenuEvent` _asf_wbp_menu_3d (delegate `MenuTransition`))
  (`self.SetActorEnableCollision` false))

(event `MenuTransition`
  (params (MenuIndex :type Integer))
  (if (`KismetArrayLibrary.Array_IsValidIndex` (`self.LinkedMenus`) MenuIndex)
    (`self.TransitionTo` (`|GetArrayItem` (`self.LinkedMenus`) MenuIndex))))

(event `TransitionTo`
  (params (NewMenu :type "/Game/Menu/BP_Menu3DActor Object Reference"))
  (`self.SetActorEnableCollision` false)
  (`self.SetActorEnableCollision` NewMenu true)
  (`PlayerController.SetViewTargetWithBlend` (`GameplayStatics.GetPlayerController` 0) NewMenu 2.0 "VTBlend_EaseInOut" 2.0 false))

(fn `UserConstructionScript`)