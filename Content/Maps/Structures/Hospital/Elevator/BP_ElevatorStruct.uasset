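; Hospital elevator Blueprint that closes its interior doors and moves the car when a BP_SwatCharacter overlaps the BoxActiveElevator trigger.
; The overlap plays a 2D sound, then drives left and right door pairs along X through four timelines, with two nested in the others' updates.
; After a one-second delay, without waiting on the door timelines, another timeline moves ElevadorStruct along Z using its ElevatorUp track.
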(event `self.BoxActiveElevator.OnComponentBeginOverlap`
  (params (OverlappedComponent :type "PrimitiveComponent Object Reference") (OtherActor :type "Actor Object Reference") (OtherComp :type "PrimitiveComponent Object Reference") (OtherBodyIndex :type Integer) (bFromSweep :type Boolean) (SweepResult :type "HitResult Structure (by ref)"))
  ;[1 1 1] Open/Close DoorInt Elevator and Up/Down
  (cast `/Game/Character/Blueprints/BP_SwatCharacter` OtherActor)
  ;;[1 0 0] Need audio
  (`GameplayStatics.PlaySound2D` null 1.0 1.0 0.0 null null)
  (`|ExecutionSequence`
    (:`then_0`
      (bind (_direction _doorintclose_r) (`Timeline|Timeline_1`)
        (:`Update`
          (`SceneComponent.K2_SetRelativeLocation` (`self.Hosp_Elev_DoorInt_R1`) (`KismetMathLibrary.MakeVector` _doorintclose_r) false false)
          (`SceneComponent.K2_SetRelativeLocation` (`self.Hosp_Elev_DoorInt_R2`) (`KismetMathLibrary.MakeVector` _doorintclose_r) false false)
          (bind (_direction_2 _doorintclose_l) (`Timeline|Timeline_4`)
            (:`Update`
              (`SceneComponent.K2_SetRelativeLocation` (`self.Hosp_Elev_DoorInt_L1`) (`KismetMathLibrary.MakeVector` _doorintclose_l) false false)
              (`SceneComponent.K2_SetRelativeLocation` (`self.Hosp_Elev_DoorInt_L2`) (`KismetMathLibrary.MakeVector` _doorintclose_l) false false))))))
    (:`then_1`
      (bind (_direction_3 _doorintclose_l_2) (`Timeline|Timeline_2`)
        (:`Update`
          (`SceneComponent.K2_SetRelativeLocation` (`self.Hosp_Elev_DoorInt_L1`) (`KismetMathLibrary.MakeVector` _doorintclose_l_2) false false)
          (`SceneComponent.K2_SetRelativeLocation` (`self.Hosp_Elev_DoorInt_L2`) (`KismetMathLibrary.MakeVector` _doorintclose_l_2) false false)
          (bind (_direction_4 _doorintclose_r_2) (`Timeline|Timeline_3`)
            (:`Update`
              (`SceneComponent.K2_SetRelativeLocation` (`self.Hosp_Elev_DoorInt_R1`) (`KismetMathLibrary.MakeVector` _doorintclose_r_2) false false)
              (`SceneComponent.K2_SetRelativeLocation` (`self.Hosp_Elev_DoorInt_R2`) (`KismetMathLibrary.MakeVector` _doorintclose_r_2) false false))))))
    (:`then_2`
      (`KismetSystemLibrary.Delay` 1.0)
      (bind (_direction_5 _elevatorup) (`Timeline|Timeline_0`)
        (:`Update`
          (`SceneComponent.K2_SetRelativeLocation` (`self.Elevador_Struct`) (`KismetMathLibrary.MakeVector` 0.0 0.0 _elevatorup) false false))))))

(fn `UserConstructionScript`)