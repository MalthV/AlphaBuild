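; Hospital elevator that opens its doors and carries the player up when a BP_SwatCharacter overlaps its trigger boxes.
; BoxFloorZero plays timelines that slide exterior and interior doors, reversing them on exit; delayed chains also drive the floor-one exterior doors.
; BoxActiveElevator raises the car structure by timeline, then moves the interior doors through separate timelines after a delay.
; Sequencing relies on Delays fired from timeline Update pins.
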(event `self.BoxFloorZero.OnComponentBeginOverlap`
  (params (OverlappedComponent :type "PrimitiveComponent Object Reference") (OtherActor :type "Actor Object Reference") (OtherComp :type "PrimitiveComponent Object Reference") (OtherBodyIndex :type Integer) (bFromSweep :type Boolean) (SweepResult :type "HitResult Structure (by ref)"))
  ;[1 1 1] Open/Close Door Elevator
  (cast `/Game/Character/Blueprints/BP_SwatCharacter` OtherActor)
  (`GameplayStatics.PlaySound2D` "/Game/Sounds/SoundEffects/OpenDoor/OpenCloseDoor.OpenCloseDoor" 1.0 1.0 0.0 null null)
  (`|ExecutionSequence`
    (:`then_0`
      (bind (_direction _opendoora) (`Timeline|DoorA_Open_Close` :!label _label)
        (:`Update`
          (`SceneComponent.K2_SetRelativeLocation` (`self.PortaElevadorP1Ext_D`) (`KismetMathLibrary.MakeVector` _opendoora) false false)
          (`SceneComponent.K2_SetRelativeLocation` (`self.Elev_DoorInt_R2`) (`KismetMathLibrary.MakeVector` _opendoora) false false)
          (`SceneComponent.K2_SetRelativeLocation` (`self.Hosp_Elev_DoorInt_R1`) (`KismetMathLibrary.MakeVector` _opendoora) false false)
          (`KismetSystemLibrary.Delay` 12.0)
          (`|ExecutionSequence`
            (:`then_0`
              ;[1 0 0] REVER
              (bind (_direction_2 _opendoora_2) (`Timeline|DoorExt_A_FloorOne_Open_Close` :!label _label_2)
                (:`Update`
                  (`SceneComponent.K2_SetRelativeLocation` (`self.PortaElevadorP1Ext_E1`) (`KismetMathLibrary.MakeVector` _opendoora_2) false false))))
            (:`then_1`
              (bind (_direction_3 _opendoorb) (`Timeline|DoorExt_B_FloorOne_Open_Close` :!label _label_3)
                (:`Update`
                  (`SceneComponent.K2_SetRelativeLocation` (`self.PortaElevadorP1Ext_D1`) (`KismetMathLibrary.MakeVector` _opendoorb) false false))))))))
    (:`then_1`
      (bind (_direction_4 _opendoorb_2) (`Timeline|DoorB_Open_Close` :!label _label_4)
        (:`Update`
          (`SceneComponent.K2_SetRelativeLocation` (`self.PortaElevadorP1Ext_E`) (`KismetMathLibrary.MakeVector` _opendoorb_2) false false)
          (`SceneComponent.K2_SetRelativeLocation` (`self.Hosp_Elev_DoorInt_L2`) (`KismetMathLibrary.MakeVector` _opendoorb_2) false false)
          (`SceneComponent.K2_SetRelativeLocation` (`self.Hosp_Elev_DoorInt_L1`) (`KismetMathLibrary.MakeVector` _opendoorb_2) false false)
          (`KismetSystemLibrary.Delay` 12.0)
          (`|ExecutionSequence`
            (:`then_0`
              (goto _label_2 :!via `Reverse`))
            (:`then_1`
              (goto _label_3 :!via `Reverse`))))))))

(event `self.BoxFloorZero.OnComponentEndOverlap`
  (params (OverlappedComponent :type "PrimitiveComponent Object Reference") (OtherActor :type "Actor Object Reference") (OtherComp :type "PrimitiveComponent Object Reference") (OtherBodyIndex :type Integer))
  ;[1 1 1] Open/Close Door Elevator
  (cast `/Game/Character/Blueprints/BP_SwatCharacter` OtherActor)
  (`GameplayStatics.PlaySound2D` "/Game/Sounds/SoundEffects/OpenDoor/OpenCloseDoor.OpenCloseDoor" 1.0 1.0 0.0 null null)
  (`|ExecutionSequence`
    (:`then_0`
      (goto _label :!via `Reverse`))
    (:`then_1`
      (goto _label_4 :!via `Reverse`))))

(event `self.BoxActiveElevator.OnComponentBeginOverlap`
  (params (OverlappedComponent :type "PrimitiveComponent Object Reference") (OtherActor :type "Actor Object Reference") (OtherComp :type "PrimitiveComponent Object Reference") (OtherBodyIndex :type Integer) (bFromSweep :type Boolean) (SweepResult :type "HitResult Structure (by ref)"))
  ;[1 1 1] Open/Close DoorExt and DoorInt of Elevator and Up
  (cast `/Game/Character/Blueprints/BP_SwatCharacter` OtherActor)
  ;;[1 0 0] Need audio
  (`GameplayStatics.PlaySound2D` null 1.0 1.0 0.0 null null)
  (`KismetSystemLibrary.Delay` 1.0)
  (bind (_direction _elevatorup) (`Timeline|ElevatorUP`)
    (:`Update`
      (`SceneComponent.K2_SetRelativeLocation` (`self.Elevador_Struct`) (`KismetMathLibrary.MakeVector` 0.0 0.0 _elevatorup) false false)
      (`KismetSystemLibrary.Delay` 5.0)
      ;[1 1 1] OPEN DOOR INT AFTER 5 SEC
      (`|ExecutionSequence`
        (:`then_0`
          (bind (_direction_2 _doorintclose_r) (`Timeline|Timeline_3`)
            (:`Update`
              (`SceneComponent.K2_SetRelativeLocation` (`self.Hosp_Elev_DoorInt_L2`) (`KismetMathLibrary.MakeVector` _doorintclose_r) false false)
              (`SceneComponent.K2_SetRelativeLocation` (`self.Hosp_Elev_DoorInt_L1`) (`KismetMathLibrary.MakeVector` _doorintclose_r) false false))))
        (:`then_1`
          (bind (_direction_3 _doorintclose_l) (`Timeline|Timeline_4`)
            (:`Update`
              (`SceneComponent.K2_SetRelativeLocation` (`self.Hosp_Elev_DoorInt_R1`) (`KismetMathLibrary.MakeVector` _doorintclose_l) false false)
              (`SceneComponent.K2_SetRelativeLocation` (`self.Elev_DoorInt_R2`) (`KismetMathLibrary.MakeVector` _doorintclose_l) false false))))))))

(fn `UserConstructionScript`)