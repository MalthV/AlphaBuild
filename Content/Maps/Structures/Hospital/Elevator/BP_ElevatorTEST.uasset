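; Test Blueprint of a two-floor hospital elevator with sliding doors, triggered by BP_SwatCharacter overlaps.
; Floor boxes flip-flop door timelines and sound, gated by InUse and floor flags.
; The cabin box toggles floor flags and plays or reverses the lift timeline on overlap, despite its "PRESS E" print, with delayed door timelines chained from its updates.
; InUse is never cleared here, and Tick prints the state for debugging.
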(event `self.BoxFloorZero.OnComponentBeginOverlap`
  (params (OverlappedComponent :type "PrimitiveComponent Object Reference") (OtherActor :type "Actor Object Reference") (OtherComp :type "PrimitiveComponent Object Reference") (OtherBodyIndex :type Integer) (bFromSweep :type Boolean) (SweepResult :type "HitResult Structure (by ref)"))
  ;[1 1 1] Open/Close Door Elevator - FLOOR ZERO
  (cast `/Game/Character/Blueprints/BP_SwatCharacter` OtherActor)
  (if (and (not (`self.In_Use`)) (`self.FloorZero`))
    (`/Engine/EditorBlueprintResources/StandardMacros.FlipFlop` :!label _label
      (:`A`
        (`GameplayStatics.PlaySound2D` "/Game/Sounds/SoundEffects/OpenDoor/OpenCloseDoor.OpenCloseDoor" 1.0 1.0 0.0 null null)
        (`|ExecutionSequence`
          (:`then_0`
            (bind (_direction _opendoora) (`Timeline|DoorA_Open_Close` :!label _label_2)
              (:`Update`
                (`SceneComponent.K2_SetRelativeLocation` (`self.PortaElevadorP1Ext_D`) (`KismetMathLibrary.MakeVector` _opendoora) false false)
                (`SceneComponent.K2_SetRelativeLocation` (`self.Elev_DoorInt_R2`) (`KismetMathLibrary.MakeVector` _opendoora) false false)
                (`SceneComponent.K2_SetRelativeLocation` (`self.Hosp_Elev_DoorInt_R1`) (`KismetMathLibrary.MakeVector` _opendoora) false false))))
          (:`then_1`
            (bind (_direction_2 _opendoorb) (`Timeline|DoorB_Open_Close` :!label _label_3)
              (:`Update`
                (`SceneComponent.K2_SetRelativeLocation` (`self.PortaElevadorP1Ext_E`) (`KismetMathLibrary.MakeVector` _opendoorb) false false)
                (`SceneComponent.K2_SetRelativeLocation` (`self.Hosp_Elev_DoorInt_L2`) (`KismetMathLibrary.MakeVector` _opendoorb) false false)
                (`SceneComponent.K2_SetRelativeLocation` (`self.Hosp_Elev_DoorInt_L1`) (`KismetMathLibrary.MakeVector` _opendoorb) false false))))))
      (:`B`
        (`GameplayStatics.PlaySound2D` "/Game/Sounds/SoundEffects/OpenDoor/OpenCloseDoor.OpenCloseDoor" 1.0 1.0 0.0 null null)
        (`|ExecutionSequence`
          (:`then_0`
            (goto _label_2 :!via `Reverse`))
          (:`then_1`
            (goto _label_3 :!via `Reverse`)))))))

(event `self.BoxFloorZero.OnComponentEndOverlap`
  (params (OverlappedComponent :type "PrimitiveComponent Object Reference") (OtherActor :type "Actor Object Reference") (OtherComp :type "PrimitiveComponent Object Reference") (OtherBodyIndex :type Integer))
  ;[1 1 1] Open/Close Door Elevator - FLOOR ZERO
  (cast `/Game/Character/Blueprints/BP_SwatCharacter` OtherActor)
  (if (not (`self.In_Use`))
    (goto _label)))

(event `self.BoxActiveElevator.OnComponentBeginOverlap`
  (params (OverlappedComponent :type "PrimitiveComponent Object Reference") (OtherActor :type "Actor Object Reference") (OtherComp :type "PrimitiveComponent Object Reference") (OtherBodyIndex :type Integer) (bFromSweep :type Boolean) (SweepResult :type "HitResult Structure (by ref)"))
  ;[1 1 1] Elevator Up
  (cast `/Game/Character/Blueprints/BP_SwatCharacter` OtherActor)
  (if (not (`self.In_Use`))
    (`KismetSystemLibrary.PrintString` "PRESS \" E\" ")
    (else
      (`KismetSystemLibrary.PrintString` "BUSY LIFT")))
  (`/Engine/EditorBlueprintResources/StandardMacros.FlipFlop`
    (:`A`
      (set `self.FloorZero` false)
      (set `self.FloorOne` true)
      (bind (_direction _elevatorup) (`Timeline|ElevatorUP` :!label _label_4)
        (:`Update`
          (set `self.In_Use` true)
          ;;[1 0 0] Need audio
          (`GameplayStatics.PlaySound2D` null 1.0 1.0 0.0 null null)
          (`KismetSystemLibrary.Delay` 1.0)
          (`SceneComponent.K2_SetRelativeLocation` (`self.Elevador_Struct`) (`KismetMathLibrary.MakeVector` 0.0 0.0 _elevatorup) false false)
          (`KismetSystemLibrary.Delay` 5.0)
          (if (`self.FloorZero`)
            ;[1 0 0] TEST
            ;;[1 1 1] OPEN DOOR INT AFTER 5 SEC
            (`|ExecutionSequence`
              (:`then_0`
                (bind (_direction_2 _doorintclose_r) (`Timeline|Timeline_2` :!via `Reverse`)
                  (:`Update`
                    (`SceneComponent.K2_SetRelativeLocation` (`self.Hosp_Elev_DoorInt_L2`) (`KismetMathLibrary.MakeVector` _doorintclose_r) false false)
                    (`SceneComponent.K2_SetRelativeLocation` (`self.Hosp_Elev_DoorInt_L1`) (`KismetMathLibrary.MakeVector` _doorintclose_r) false false)
                    (`SceneComponent.K2_SetRelativeLocation` (`self.PortaElevadorP1Ext_E1`) (`KismetMathLibrary.MakeVector` _doorintclose_r) false false))))
              (:`then_1`
                (bind (_direction_3 _doorintclose_l) (`Timeline|Timeline_5` :!via `Reverse`)
                  (:`Update`
                    (`SceneComponent.K2_SetRelativeLocation` (`self.Hosp_Elev_DoorInt_R1`) (`KismetMathLibrary.MakeVector` _doorintclose_l) false false)
                    (`SceneComponent.K2_SetRelativeLocation` (`self.Elev_DoorInt_R2`) (`KismetMathLibrary.MakeVector` _doorintclose_l) false false)
                    (`SceneComponent.K2_SetRelativeLocation` (`self.PortaElevadorP1Ext_D1`) (`KismetMathLibrary.MakeVector` _doorintclose_l) false false)))))
            (`KismetSystemLibrary.Delay` 5.0)
            ;;[1 1 1] OPEN DOOR INT AFTER 5 SEC
            (`|ExecutionSequence`
              (:`then_0`
                (bind (_direction_4 _doorintclose_r_2) (`Timeline|Timeline_6`)
                  (:`Update`
                    (`SceneComponent.K2_SetRelativeLocation` (`self.Hosp_Elev_DoorInt_L2`) (`KismetMathLibrary.MakeVector` _doorintclose_r_2) false false)
                    (`SceneComponent.K2_SetRelativeLocation` (`self.Hosp_Elev_DoorInt_L1`) (`KismetMathLibrary.MakeVector` _doorintclose_r_2) false false)
                    (`SceneComponent.K2_SetRelativeLocation` (`self.PortaElevadorP1Ext_E1`) (`KismetMathLibrary.MakeVector` _doorintclose_r_2) false false))))
              (:`then_1`
                (bind (_direction_5 _doorintclose_l_2) (`Timeline|Timeline_7`)
                  (:`Update`
                    (`SceneComponent.K2_SetRelativeLocation` (`self.Hosp_Elev_DoorInt_R1`) (`KismetMathLibrary.MakeVector` _doorintclose_l_2) false false)
                    (`SceneComponent.K2_SetRelativeLocation` (`self.Elev_DoorInt_R2`) (`KismetMathLibrary.MakeVector` _doorintclose_l_2) false false)
                    (`SceneComponent.K2_SetRelativeLocation` (`self.PortaElevadorP1Ext_D1`) (`KismetMathLibrary.MakeVector` _doorintclose_l_2) false false)))))
            (else
              ;;[1 1 1] OPEN DOOR INT AFTER 5 SEC
              (`|ExecutionSequence`
                (:`then_0`
                  (bind (_direction_6 _doorintclose_r_3) (`Timeline|Timeline_3`)
                    (:`Update`
                      (`SceneComponent.K2_SetRelativeLocation` (`self.Hosp_Elev_DoorInt_L2`) (`KismetMathLibrary.MakeVector` _doorintclose_r_3) false false)
                      (`SceneComponent.K2_SetRelativeLocation` (`self.Hosp_Elev_DoorInt_L1`) (`KismetMathLibrary.MakeVector` _doorintclose_r_3) false false)
                      (`SceneComponent.K2_SetRelativeLocation` (`self.PortaElevadorP1Ext_E1`) (`KismetMathLibrary.MakeVector` _doorintclose_r_3) false false))))
                (:`then_1`
                  (bind (_direction_7 _doorintclose_l_3) (`Timeline|Timeline_4`)
                    (:`Update`
                      (`SceneComponent.K2_SetRelativeLocation` (`self.Hosp_Elev_DoorInt_R1`) (`KismetMathLibrary.MakeVector` _doorintclose_l_3) false false)
                      (`SceneComponent.K2_SetRelativeLocation` (`self.Elev_DoorInt_R2`) (`KismetMathLibrary.MakeVector` _doorintclose_l_3) false false)
                      (`SceneComponent.K2_SetRelativeLocation` (`self.PortaElevadorP1Ext_D1`) (`KismetMathLibrary.MakeVector` _doorintclose_l_3) false false)))))
              (`KismetSystemLibrary.Delay` 5.0)
              ;;[1 1 1] OPEN DOOR INT AFTER 5 SEC
              (`|ExecutionSequence`
                (:`then_0`
                  (bind (_direction_8 _doorintclose_r_4) (`Timeline|Timeline_8` :!via `Reverse`)
                    (:`Update`
                      (`SceneComponent.K2_SetRelativeLocation` (`self.Hosp_Elev_DoorInt_L2`) (`KismetMathLibrary.MakeVector` _doorintclose_r_4) false false)
                      (`SceneComponent.K2_SetRelativeLocation` (`self.Hosp_Elev_DoorInt_L1`) (`KismetMathLibrary.MakeVector` _doorintclose_r_4) false false)
                      (`SceneComponent.K2_SetRelativeLocation` (`self.PortaElevadorP1Ext_E1`) (`KismetMathLibrary.MakeVector` _doorintclose_r_4) false false))))
                (:`then_1`
                  (bind (_direction_9 _doorintclose_l_4) (`Timeline|Timeline_9` :!via `Reverse`)
                    (:`Update`
                      (`SceneComponent.K2_SetRelativeLocation` (`self.Hosp_Elev_DoorInt_R1`) (`KismetMathLibrary.MakeVector` _doorintclose_l_4) false false)
                      (`SceneComponent.K2_SetRelativeLocation` (`self.Elev_DoorInt_R2`) (`KismetMathLibrary.MakeVector` _doorintclose_l_4) false false)
                      (`SceneComponent.K2_SetRelativeLocation` (`self.PortaElevadorP1Ext_D1`) (`KismetMathLibrary.MakeVector` _doorintclose_l_4) false false))))))))))
    (:`B`
      (set `self.FloorZero` true)
      (set `self.FloorOne` false)
      (goto _label_4 :!via `Reverse`))))

(event `self.ReceiveTick`
  (params (DeltaSeconds :type "Float (single-precision)"))
  (`KismetSystemLibrary.PrintString` (`KismetStringLibrary.Conv_BoolToString` (`self.In_Use`)))
  (`KismetSystemLibrary.PrintString` (`KismetStringLibrary.Conv_BoolToString` (`self.FloorZero`)) true true (struct :`G` 1.0 :`B` 0.261176 :`A` 1.0))
  (`KismetSystemLibrary.PrintString` (`KismetStringLibrary.Conv_BoolToString` (`self.FloorOne`)) true true (struct :`R` 1.0 :`B` 0.100676 :`A` 1.0)))

(event `self.BoxFloorOne.OnComponentBeginOverlap`
  (params (OverlappedComponent :type "PrimitiveComponent Object Reference") (OtherActor :type "Actor Object Reference") (OtherComp :type "PrimitiveComponent Object Reference") (OtherBodyIndex :type Integer) (bFromSweep :type Boolean) (SweepResult :type "HitResult Structure (by ref)"))
  ;[1 1 1] Open/Close Door Elevator - FLOOR ONE
  (cast `/Game/Character/Blueprints/BP_SwatCharacter` OtherActor)
  (if (and (not (`self.In_Use`)) (`self.FloorOne`))
    (`/Engine/EditorBlueprintResources/StandardMacros.FlipFlop` :!label _label_5
      (:`A`
        (`GameplayStatics.PlaySound2D` "/Game/Sounds/SoundEffects/OpenDoor/OpenCloseDoor.OpenCloseDoor" 1.0 1.0 0.0 null null)
        (`|ExecutionSequence`
          (:`then_0`
            (bind (_direction _opendoora) (`Timeline|Timeline_0` :!label _label_6)
              (:`Update`
                (`SceneComponent.K2_SetRelativeLocation` (`self.PortaElevadorP1Ext_D`) (`KismetMathLibrary.MakeVector` _opendoora) false false)
                (`SceneComponent.K2_SetRelativeLocation` (`self.Elev_DoorInt_R2`) (`KismetMathLibrary.MakeVector` _opendoora) false false)
                (`SceneComponent.K2_SetRelativeLocation` (`self.Hosp_Elev_DoorInt_R1`) (`KismetMathLibrary.MakeVector` _opendoora) false false))))
          (:`then_1`
            (bind (_direction_2 _opendoorb) (`Timeline|Timeline_1` :!label _label_7)
              (:`Update`
                (`SceneComponent.K2_SetRelativeLocation` (`self.PortaElevadorP1Ext_E`) (`KismetMathLibrary.MakeVector` _opendoorb) false false)
                (`SceneComponent.K2_SetRelativeLocation` (`self.Hosp_Elev_DoorInt_L2`) (`KismetMathLibrary.MakeVector` _opendoorb) false false)
                (`SceneComponent.K2_SetRelativeLocation` (`self.Hosp_Elev_DoorInt_L1`) (`KismetMathLibrary.MakeVector` _opendoorb) false false))))))
      (:`B`
        (`GameplayStatics.PlaySound2D` "/Game/Sounds/SoundEffects/OpenDoor/OpenCloseDoor.OpenCloseDoor" 1.0 1.0 0.0 null null)
        (`|ExecutionSequence`
          (:`then_0`
            (goto _label_6 :!via `Reverse`))
          (:`then_1`
            (goto _label_7 :!via `Reverse`)))))))

(event `self.BoxFloorOne.OnComponentEndOverlap`
  (params (OverlappedComponent :type "PrimitiveComponent Object Reference") (OtherActor :type "Actor Object Reference") (OtherComp :type "PrimitiveComponent Object Reference") (OtherBodyIndex :type Integer))
  ;[1 1 1] Open/Close Door Elevator - FLOOR ONE
  (cast `/Game/Character/Blueprints/BP_SwatCharacter` OtherActor)
  (if (not (`self.In_Use`))
    (goto _label_5)))

(fn `UserConstructionScript`)