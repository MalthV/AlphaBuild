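; Hospital structure Blueprint with two automatic sliding double doors between Screening and FrontDeck.
; When a BP_SwatCharacter enters a door's collision box, a 2D open/close sound plays and two timelines slide that door's leaves apart along local X.
; Leaving the box plays the sound again and reverses both timelines to close it.
; Each door has its own box and timelines, and the construction script is empty.
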(event `self.BoxCollisionDoorA1m.OnComponentBeginOverlap`
  (params (OverlappedComponent :type "PrimitiveComponent Object Reference") (OtherActor :type "Actor Object Reference") (OtherComp :type "PrimitiveComponent Object Reference") (OtherBodyIndex :type Integer) (bFromSweep :type Boolean) (SweepResult :type "HitResult Structure (by ref)"))
  ;[1 1 1] Open/Close Door A 1m (Screening - FrontDeck)
  (cast `/Game/Character/Blueprints/BP_SwatCharacter` OtherActor)
  (`GameplayStatics.PlaySound2D` "/Game/Sounds/SoundEffects/OpenDoor/OpenCloseDoor.OpenCloseDoor" 1.0 1.0 0.0 null null)
  (`|ExecutionSequence`
    (:`then_0`
      (bind (_direction _opendoora) (`Timeline|OpenDoorA` :!label _label)
        (:`Update`
          (`SceneComponent.K2_SetRelativeLocation` (`self.DoorSci-Fy_A1m_DoorA`) (`KismetMathLibrary.MakeVector` _opendoora) false false))))
    (:`then_1`
      (bind (_direction_2 _opendoorb) (`Timeline|OpenDoorB` :!label _label_2)
        (:`Update`
          (`SceneComponent.K2_SetRelativeLocation` (`self.DoorSci-Fy_A1m_DoorB`) (`KismetMathLibrary.MakeVector` _opendoorb) false false))))))

(event `self.BoxCollisionDoorA1m.OnComponentEndOverlap`
  (params (OverlappedComponent :type "PrimitiveComponent Object Reference") (OtherActor :type "Actor Object Reference") (OtherComp :type "PrimitiveComponent Object Reference") (OtherBodyIndex :type Integer))
  ;[1 1 1] Open/Close Door A 1m (Screening - FrontDeck)
  (cast `/Game/Character/Blueprints/BP_SwatCharacter` OtherActor)
  (`GameplayStatics.PlaySound2D` "/Game/Sounds/SoundEffects/OpenDoor/OpenCloseDoor.OpenCloseDoor" 1.0 1.0 0.0 null null)
  (`|ExecutionSequence`
    (:`then_0`
      (goto _label :!via `Reverse`))
    (:`then_1`
      (goto _label_2 :!via `Reverse`))))

(event `self.BoxCollisionDoorA1m1.OnComponentBeginOverlap`
  (params (OverlappedComponent :type "PrimitiveComponent Object Reference") (OtherActor :type "Actor Object Reference") (OtherComp :type "PrimitiveComponent Object Reference") (OtherBodyIndex :type Integer) (bFromSweep :type Boolean) (SweepResult :type "HitResult Structure (by ref)"))
  ;[1 1 1] Open/Close Door B 1m (Screening - FrontDeck)
  (cast `/Game/Character/Blueprints/BP_SwatCharacter` OtherActor)
  (`GameplayStatics.PlaySound2D` "/Game/Sounds/SoundEffects/OpenDoor/OpenCloseDoor.OpenCloseDoor" 1.0 1.0 0.0 null null)
  (`|ExecutionSequence`
    (:`then_0`
      (bind (_direction _opendoora) (`Timeline|Timeline_0` :!label _label_3)
        (:`Update`
          (`SceneComponent.K2_SetRelativeLocation` (`self.DoorSci-Fy_A1m_DoorA1`) (`KismetMathLibrary.MakeVector` _opendoora) false false))))
    (:`then_1`
      (bind (_direction_2 _opendoorb) (`Timeline|Timeline_1` :!label _label_4)
        (:`Update`
          (`SceneComponent.K2_SetRelativeLocation` (`self.DoorSci-Fy_A1m_DoorB1`) (`KismetMathLibrary.MakeVector` _opendoorb) false false))))))

(event `self.BoxCollisionDoorA1m1.OnComponentEndOverlap`
  (params (OverlappedComponent :type "PrimitiveComponent Object Reference") (OtherActor :type "Actor Object Reference") (OtherComp :type "PrimitiveComponent Object Reference") (OtherBodyIndex :type Integer))
  ;[1 1 1] Open/Close Door B 1m (Screening - FrontDeck)
  (cast `/Game/Character/Blueprints/BP_SwatCharacter` OtherActor)
  (`GameplayStatics.PlaySound2D` "/Game/Sounds/SoundEffects/OpenDoor/OpenCloseDoor.OpenCloseDoor" 1.0 1.0 0.0 null null)
  (`|ExecutionSequence`
    (:`then_0`
      (goto _label_3 :!via `Reverse`))
    (:`then_1`
      (goto _label_4 :!via `Reverse`))))

(fn `UserConstructionScript`)