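; Rifle ammo pickup that grants a magazine to the SWAT character's Darkness rifle.
; When a BP_SwatCharacter overlaps its box collision, it destroys itself and increments the rifle's MaxMag, capped at three.
; The resulting MaxMag is printed to screen as debug output.
; The pickup is consumed even if the rifle is already at the cap.
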(event `self.BoxCollision.OnComponentBeginOverlap`
  (params (OverlappedComponent :type "PrimitiveComponent Object Reference") (OtherActor :type "Actor Object Reference") (OtherComp :type "PrimitiveComponent Object Reference") (OtherBodyIndex :type Integer) (bFromSweep :type Boolean) (SweepResult :type "HitResult Structure (by ref)"))
  (bind _asbp_swat_character (cast `/Game/Character/Blueprints/BP_SwatCharacter` OtherActor))
  (`self.K2_DestroyActor`)
  (bind _bp_darknessrifle (`/Game/Character/Blueprints/BP_SwatCharacter.BP_DarknessRifle` _asbp_swat_character))
  (bind _maxmag (`/Game/Weapons/BP_Weapons.MaxMag` _bp_darknessrifle))
  (`/Engine/EditorBlueprintResources/StandardMacros.IncrementInt` _maxmag
    (:`  `
      (if (> _maxmag 3)
        (bind _output_get (set `/Game/Weapons/BP_Weapons.MaxMag` 3 _bp_darknessrifle))
        (`KismetSystemLibrary.PrintString` (`KismetStringLibrary.Conv_IntToString` _output_get))
        (else
          (`KismetSystemLibrary.PrintString` (`KismetStringLibrary.Conv_IntToString` _output_get)))))))

(fn `UserConstructionScript`)