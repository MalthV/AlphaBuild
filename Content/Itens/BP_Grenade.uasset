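; BP_Grenade is a thrown grenade actor that explodes on a three-second fuse.
; On BeginPlay it applies an impulse to its mesh from the player character's forward direction, scaled by an X-only vector, so only world X survives.
; After the delay it fires a radial force impulse, spawns an explosion emitter and destroys itself.
; Tick caches the Arrow component's world location as the emitter's spawn point.
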(event `self.ReceiveBeginPlay`
  (bind _returnvalue (`GameplayStatics.GetPlayerCharacter` 0))
  (`PrimitiveComponent.AddImpulseAtLocation` (`self.GranadeMash`) (* (+ (`self.GetActorForwardVector` _returnvalue) (`KismetMathLibrary.Conv_RotatorToVector` (`self.K2_GetActorRotation` _returnvalue))) (2000.0 0.0 0.0)) (`self.K2_GetActorLocation`) "None")
  (`KismetSystemLibrary.Delay` 3.0)
  (`RadialForceComponent.FireImpulse` (`self.RadialForce`))
  (`GameplayStatics.SpawnEmitterAtLocation` "/Game/SciFiWeapDark/FX/Particles/P_Grenade_Explosion_Dark.P_Grenade_Explosion_Dark" (`self.GranadeLocation`))
  (`self.K2_DestroyActor`))

(event `self.ReceiveTick`
  (params (DeltaSeconds :type "Float (single-precision)"))
  (set `self.GranadeLocation` (`SceneComponent.K2_GetComponentLocation` (`self.Arrow`))))

(fn `UserConstructionScript`)