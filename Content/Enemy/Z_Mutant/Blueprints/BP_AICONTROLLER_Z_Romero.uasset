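; AI controller for the Z_Romero mutant enemy, which starts the BT_Z_Romero behavior tree on BeginPlay.
; AI Perception updates the CanSeePlayer blackboard key whenever sensing of a BP_SwatCharacter changes.
; Walk and Run events forward to ZRomeroPawn, but the logic that assigns that pawn and the PathLooping key is disconnected and never runs.
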(event `self.ReceiveBeginPlay`
  (`self.RunBehaviorTree` "/Game/Enemy/Z_Mutant/Blueprints/AI/BT_Z_Romero.BT_Z_Romero"))

(event `self.AIPerception.OnTargetPerceptionUpdated`
  (params (Actor :type "Actor Object Reference") (Stimulus :type "AIStimulus Structure"))
  (cast `/Game/Character/Blueprints/BP_SwatCharacter` Actor)
  (`BlackboardComponent.SetValueAsBool` (`AIBlueprintHelperLibrary.GetBlackboard` null) "CanSeePlayer" Stimulus_bSuccessfullySensed))

(event `Walk`
  (`/Game/Enemy/Z_Mutant/Blueprints/BP_Z_Romero.Walk` (`self.Z Romero Pawn`)))

(event `Run`
  (`/Game/Enemy/Z_Mutant/Blueprints/BP_Z_Romero.Run` (`self.Z Romero Pawn`)))

(fn `UserConstructionScript`)