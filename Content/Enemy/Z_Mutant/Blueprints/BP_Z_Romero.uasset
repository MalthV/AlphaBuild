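; BP_Z_Romero is a mutant zombie enemy character that sets its health to maximum at BeginPlay.
; Run and Walk events switch its movement speed.
; A mesh hit at zero or lower health destroys the capsule, then the actor after a short delay.
; The damage and ragdoll death logic is disconnected and TakeDamage is empty, so nothing here lowers health.
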(event `self.ReceiveBeginPlay`
  (set `self.CurrentHealth` (`self.MaxHealth`)))

(event `self.ReceiveActorBeginOverlap`
  (params (OtherActor :type "Actor Object Reference")))

(event `/Game/Enemy/BPI_DamageSystem.TakeDamage`
  (params (BoneName :type Name) (Damage :type "Float (single-precision)")))

(event `Run`
  (set `CharacterMovementComponent.MaxWalkSpeed` 600.0 (`self.CharacterMovement`)))

(event `Walk`
  (set `CharacterMovementComponent.MaxWalkSpeed` 100.0 (`self.CharacterMovement`)))

(event `self.Mesh.OnComponentHit`
  (params (HitComponent :type "PrimitiveComponent Object Reference") (OtherActor :type "Actor Object Reference") (OtherComp :type "PrimitiveComponent Object Reference") (NormalImpulse :type "Vector Structure") (Hit :type "HitResult Structure (by ref)"))
  (if (<= (`self.CurrentHealth`) 0.0)
    (`/Engine/EditorBlueprintResources/StandardMacros.IsValid` (`self.CapsuleComponent`)
      (:`Is Valid`
        (`ActorComponent.K2_DestroyComponent` (`self.CapsuleComponent`))
        (`KismetSystemLibrary.Delay` 2.0)
        (`self.K2_DestroyActor`)))))

(fn `UserConstructionScript`)