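; BP_BadCubeActor is a hazard cube that damages the SWAT character when it enters the cube's collision.
; On overlap it stores the character and calls DoDamage, then continues into the same damage logic, so that logic runs twice per overlap.
; The logic calls ApplyDamage, subtracts the returned amount directly from the character's HealthAmount and prints the remaining health.
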(event `self.BadCubeCollision.OnComponentBeginOverlap`
  (params (OverlappedComponent :type "PrimitiveComponent Object Reference") (OtherActor :type "Actor Object Reference") (OtherComp :type "PrimitiveComponent Object Reference") (OtherBodyIndex :type Integer) (bFromSweep :type Boolean) (SweepResult :type "HitResult Structure (by ref)"))
  (bind _bp_swatcharacter (`self.BP_SwatCharacter`))
  (bind _asbp_swat_character (cast `/Game/Character/Blueprints/BP_SwatCharacter` OtherActor))
  (bind _output_get (set `self.BP_SwatCharacter` _asbp_swat_character))
  (`self.DoDamage`)
  (bind _returnvalue (`GameplayStatics.ApplyDamage` _output_get (`self.Damage`) :!label _label))
  (bind _output_get_2 (set `/Game/Character/Blueprints/BP_SwatCharacter.HealthAmount` (- (`/Game/Character/Blueprints/BP_SwatCharacter.HealthAmount` _bp_swatcharacter) _returnvalue) _bp_swatcharacter))
  (`KismetSystemLibrary.PrintString` (`KismetStringLibrary.Conv_DoubleToString` _output_get_2)))

(event `DoDamage`
  (goto _label))

(fn `UserConstructionScript`)