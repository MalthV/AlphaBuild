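; BP_Bip is a life monitor screen that reflects the player's health through color.
; It opens the Sinapces media source on BeginPlay, then polls BP_SwatCharacter health every Tick.
; Moderate and critical health bands play timelines that scale green or red vectors from MParam_RGBADITIVE into the RGB parameter of MParam_RGBNeural.
; At zero health, the screen mesh switches to the black synapse material, M_SinapsesPreto.
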(event `self.ReceiveBeginPlay`
  (`MediaPlayer.OpenSource` (`self.MP_Sinapses`) "/Game/HUD/LifeMonitorVideoTextures/Sinapces.Sinapces"))

(event `self.ReceiveTick`
  (params (DeltaSeconds :type "Float (single-precision)"))
  (bind _healthamount (`/Game/Character/Blueprints/BP_SwatCharacter.HealthAmount` (cast `/Game/Character/Blueprints/BP_SwatCharacter` (`GameplayStatics.GetPlayerCharacter` 0) :!pure true)))
  (`|ExecutionSequence`
    (:`then_0`
      (if (and (<= _healthamount 60.0) (> _healthamount 20.0))
        (bind _returnvalue (`KismetMaterialLibrary.GetVectorParameterValue` "/Game/HUD/LifeMonitor/Materials/MParam_RGBADITIVE.MParam_RGBADITIVE" "VectorGREEN"))
        (bind (_direction _decreaseamount) (`Timeline|HealthDecreaseTimelineGreen`)
          (:`Update`
            (`KismetMaterialLibrary.SetVectorParameterValue` "/Game/HUD/LifeMonitor/Materials/MParam_RGBNeural.MParam_RGBNeural" "RGB_VectorParam" (* _returnvalue _decreaseamount))))))
    (:`then_1`
      (if (<= _healthamount 20.0)
        (bind _returnvalue_2 (`KismetMaterialLibrary.GetVectorParameterValue` "/Game/HUD/LifeMonitor/Materials/MParam_RGBADITIVE.MParam_RGBADITIVE" "VectorRED"))
        (bind (_direction_2 _decreaseamount_2) (`Timeline|HealtDecreaseAmountRed`)
          (:`Update`
            (`KismetMaterialLibrary.SetVectorParameterValue` "/Game/HUD/LifeMonitor/Materials/MParam_RGBNeural.MParam_RGBNeural" "RGB_VectorParam" (* _returnvalue_2 _decreaseamount_2))))))
    (:`then_2`
      (if (<= _healthamount 0.0)
        (`PrimitiveComponent.SetMaterial` (`self.BIP_Bip_Tela`) 0 "/Game/HUD/LifeMonitor/Materials/M_SinapsesPreto.M_SinapsesPreto")))))

(fn `UserConstructionScript`)