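; Sci-fi rifle weapon that handles firing, ammo and a laser sight.
; Fire decrements ammo, flagging the player's SWAT character to reload at zero, then line-traces to aim a spawned projectile.
; The trace itself applies bone-based damage through BPI_DamageSystem and breaks the hit bone's constraint on BP_Z_FemaleTest.
; Tick updates the beam and spawns an end emitter each frame if the beam exists; its spawn call in EventGraph is unwired.
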(event `self.Fire`
  (`self.AmmoCounter`)
  (`self.ShootLineTrace`))

(event `self.ReceiveBeginPlay`)

(event `self.ReceiveTick`
  (params (DeltaSeconds :type "Float (single-precision)"))
  (`self.LaserBeamFunction` DeltaSeconds))

(fn `AmmoCounter`
  (bind _asbp_swat_character (cast `/Game/Character/Blueprints/BP_SwatCharacter` (`GameplayStatics.GetPlayerCharacter` 0) :!pure true))
  ;[1 1 1] If ammo >0 decreace until reach 0, the set shooting as false and reloading as true
  (if (> (`self.AmmoCount`) 0)
    (bind _result (`/Engine/EditorBlueprintResources/StandardMacros.DecrementInt` (`self.AmmoCount`))
      (:`  `
        (if (== _result 0)
          (set `/Game/Character/Blueprints/BP_SwatCharacter.IsShooting` false _asbp_swat_character)
          (set `/Game/Character/Blueprints/BP_SwatCharacter.IsReloading` true _asbp_swat_character))))))

(fn `CalculateDamage`
  (params (BoneName :type Name))
  (returns (DamageValue :type "Float (double-precision)"))
  (locals (Damage :type "Float (double-precision)"))
  (`|ExecutionSequence`
    (:`then_0`
      (if (or (== BoneName "Head") (== BoneName "LeftForeArm") (== BoneName "LeftHand") (== BoneName "LeftLeg") (== BoneName "LeftFoot") (== BoneName "RightForeArm") (== BoneName "RightHand") (== BoneName "RightLeg") (== BoneName "RightFoot"))
        (bind _output_get (set `local.Damage` 30.0))
        (return _output_get)
        (else
          (bind _output_get_2 (set `local.Damage` 10.0))
          (return _output_get_2))))))

(fn `LaserBeamFunction`
  (params (DrawTime :type "Float (double-precision)"))
  (bind _laserarrow (`self.LaserArrow`))
  (bind _returnvalue (`SceneComponent.K2_GetComponentLocation` _laserarrow))
  (`/Engine/EditorBlueprintResources/StandardMacros.IsValid` (`self.LaserParticle`)
    (:`Is Valid`
      (`ParticleSystemComponent.SetBeamSourcePoint` (`self.LaserParticle`) 0 _returnvalue 0)
      (bind _outhit (`KismetSystemLibrary.LineTraceSingle` :`Start` _returnvalue :`End` (+ _returnvalue (* (`SceneComponent.GetForwardVector` _laserarrow) 250000.0)) :`TraceChannel` "TraceTypeQuery1" :`DrawTime` DrawTime))
      (bind (_bblockinghit _binitialoverlap _time _distance _location _impactpoint _normal _impactnormal _physmat _hitactor _hitcomponent _hitbonename _hititem _faceindex _tracestart _traceend) (`GameplayStatics.BreakHitResult` _outhit))
      (bind _returnvalue_2 (`KismetMathLibrary.SelectVector` _location _traceend _bblockinghit))
      (`ParticleSystemComponent.SetBeamTargetPoint` (`self.LaserParticle`) 0 _returnvalue_2 0)
      (bind _output_get (set `self.HitResultEndLocation` _returnvalue_2))
      (bind _returnvalue_3 (`GameplayStatics.SpawnEmitterAtLocation` "/Game/SciFiWeapDark/FX/Particles/LazerEnd.LazerEnd" _output_get (struct) (0.2 0.2 0.2)))
      (set `self.LaserEnd` _returnvalue_3))))

(fn `LaserBeamSpawn`
  (bind _returnvalue (`GameplayStatics.SpawnEmitterAttached` "/Game/Weapons/P_Beam.P_Beam" (`self.LaserArrow`) "None" (0.0 0.0 0.0) (struct) (1.0 1.0 1.0) "SnapToTarget"))
  (set `self.LaserParticle` _returnvalue))

(fn `ShootLineTrace`
  (bind _hit_bone_name (`self.Hit Bone Name`))
  (bind _laserarrow (`self.LaserArrow`))
  (bind _returnvalue (`SceneComponent.K2_GetComponentLocation` (`self.Arrow`)))
  (bind (_outhit _returnvalue_2) (`KismetSystemLibrary.LineTraceSingle` (`SceneComponent.K2_GetComponentLocation` (`self.Arrow`)) (+ (`SceneComponent.K2_GetComponentLocation` _laserarrow) (* (`SceneComponent.GetForwardVector` _laserarrow) 25000.0)) "TraceTypeQuery1"))
  (bind (_bblockinghit _binitialoverlap _time _distance _location _impactpoint _normal _impactnormal _physmat _hitactor _hitcomponent _hitbonename _hititem _faceindex _tracestart _traceend) (`GameplayStatics.BreakHitResult` _outhit))
  (set `self.Location` _location)
  (set `self.Impact Point` _impactpoint)
  (bind _output_get (set `self.Impact Normal` _impactnormal))
  (bind _output_get_2 (set `self.Hit Actor` _hitactor))
  (set `self.Hit Component` _hitcomponent)
  (set `self.Hit Bone Name` _hitbonename)
  (set `self.Trace Start` _tracestart)
  (bind _output_get_3 (set `self.Trace End` _traceend))
  (set `self.HitNormalRotation` (`KismetMathLibrary.Conv_VectorToRotator` _output_get))
  (set `self.HitActorClass` (`GameplayStatics.GetObjectClass` _output_get_2))
  (`|SpawnActorFromClass` "/Game/Weapons/BP_ScifiRifleProjectile.BP_ScifiRifleProjectile_C" (`KismetMathLibrary.MakeTransform` _returnvalue (`KismetMathLibrary.FindLookAtRotation` _returnvalue (`KismetMathLibrary.SelectVector` (`self.Impact Point`) _output_get_3 _returnvalue_2))) "AlwaysSpawn" "OverrideRootScale" null null)
  (if (`KismetSystemLibrary.DoesImplementInterface` (`self.Hit Actor`) "/Game/Enemy/BPI_DamageSystem.BPI_DamageSystem_C")
    (bind _damagevalue (`self.CalculateDamage` (`self.Hit Bone Name`)))
    (message `/Game/Enemy/BPI_DamageSystem.TakeDamage` (`self.Hit Actor`) (`self.Hit Bone Name`) _damagevalue)
    (bind _asbp_z_female_test (cast `/Game/Enemy/Z_FemaleTest/BP_Z_FemaleTest` (`self.Hit Actor`)))
    (`SkeletalMeshComponent.BreakConstraint` (`Character.Mesh` _asbp_z_female_test) (100.0 100.0 100.0) (`self.Impact Point`) _hit_bone_name)
    (`KismetSystemLibrary.PrintString` (`KismetStringLibrary.Conv_NameToString` _hit_bone_name))))

(fn `UserConstructionScript`
  (`parent.UserConstructionScript`)
  (set `self.AmmoCount` (`self.AmmoCount`))
  (set `self.MaxAmmo` (`self.MaxAmmo`)))