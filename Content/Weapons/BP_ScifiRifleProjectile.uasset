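; BP_ScifiRifleProjectile is a rifle projectile that damages BP_Z_Romero characters and expires after a few seconds.
; Any mesh hit destroys it; sphere collision hits also destroy it, then subtract fixed health directly from the Romero and print the result.
; At near-zero health it flags the Romero dead, enables mesh physics and destroys its capsule.
; TakeDamage jumps into the same sphere-hit chain, reusing that event's OtherActor.
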(event `self.ReceiveBeginPlay`
  (`self.SetLifeSpan` 3.0))

(event `self.StaticMesh.OnComponentHit`
  (params (HitComponent :type "PrimitiveComponent Object Reference") (OtherActor :type "Actor Object Reference") (OtherComp :type "PrimitiveComponent Object Reference") (NormalImpulse :type "Vector Structure") (Hit :type "HitResult Structure (by ref)"))
  (`self.K2_DestroyActor`))

(event `self.SphereCollision.OnComponentHit`
  (params (HitComponent :type "PrimitiveComponent Object Reference") (OtherActor :type "Actor Object Reference") (OtherComp :type "PrimitiveComponent Object Reference") (NormalImpulse :type "Vector Structure") (Hit :type "HitResult Structure (by ref)"))
  (bind _as_bp_z_romero (`self.As BP Z Romero`))
  (`self.K2_DestroyActor` :!label _label)
  (bind _asbp_z_romero (cast `/Game/Enemy/Z_Mutant/Blueprints/BP_Z_Romero` OtherActor))
  (bind _output_get (set `self.As BP Z Romero` _asbp_z_romero))
  (bind _currenthealth (`/Game/Enemy/Z_Mutant/Blueprints/BP_Z_Romero.CurrentHealth` _asbp_z_romero))
  (bind _output_get_2 (set `/Game/Enemy/Z_Mutant/Blueprints/BP_Z_Romero.CurrentHealth` (- _currenthealth 20.0) _output_get))
  (`KismetSystemLibrary.PrintString` (`KismetStringLibrary.Conv_DoubleToString` _output_get_2))
  (if (<= _currenthealth 1.0)
    (set `/Game/Enemy/Z_Mutant/Blueprints/BP_Z_Romero.IsDead` true _as_bp_z_romero)
    (`PrimitiveComponent.SetSimulatePhysics` (`Character.Mesh` _as_bp_z_romero) true)
    (`ActorComponent.K2_DestroyComponent` (`Character.CapsuleComponent` _as_bp_z_romero))))

(event `/Game/Enemy/BPI_DamageSystem.TakeDamage`
  (params (BoneName :type Name) (Damage :type "Float (single-precision)"))
  (goto _label))

(fn `UserConstructionScript`)