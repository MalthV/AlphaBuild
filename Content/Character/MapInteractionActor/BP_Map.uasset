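; BP_Map is a map interaction actor that updates which of its four location components are shown in game.
; MapLocationUpdate takes a pickup tag (far, medium or near) and hides a progressively larger set of those components, with near hiding all four.
; It only hides components and never shows them again; BeginPlay, Tick and the construction script are empty, so the update relies on an external call.
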(event `self.ReceiveBeginPlay`)

(fn `MapLocationUpdate`
  (params (Tag :type Name))
  (if (== Tag "FarPickUp")
    (`SceneComponent.SetHiddenInGame` (`self.Location1`) true false)
    (`SceneComponent.SetHiddenInGame` (`self.Location2`) true false)
    (elif (== Tag "MediumPickUp")
      (`SceneComponent.SetHiddenInGame` (`self.Location3`) true false)
      (`SceneComponent.SetHiddenInGame` (`self.Location2`) true false)
      (`SceneComponent.SetHiddenInGame` (`self.Location1`) true false)
      (elif (== Tag "NearPickUp")
        (`SceneComponent.SetHiddenInGame` (`self.Location4`) true false)
        (`SceneComponent.SetHiddenInGame` (`self.Location1`) true false)
        (`SceneComponent.SetHiddenInGame` (`self.Location2`) true false)
        (`SceneComponent.SetHiddenInGame` (`self.Location3`) true false)))))

(fn `UserConstructionScript`)