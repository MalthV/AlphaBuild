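; Player SWAT character that spawns and attaches a sci-fi rifle and handles movement, combat, inventory and elevator-button input.
; FlipFlops toggle stance, walk, aim laser, flashlight and inventory, with parallel SR_ events for many actions; timelines drive leaning and FOV zoom.
; A gate with a retriggerable delay loops automatic fire, while reload and grenade input only set flags.
; Line traces measure walls to choose vault or climb montages.
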(event `InputAction|FreeLook`
  (params (Key :type "Key Structure"))
  (bind _charactermovement (`self.CharacterMovement`))
  (:`Pressed`
    (set `CharacterMovementComponent.bOrientRotationToMovement` false _charactermovement)
    (set `self.bUseControllerRotationYaw` false))
  (:`Released`
    (set `CharacterMovementComponent.bOrientRotationToMovement` true _charactermovement)
    (set `self.bUseControllerRotationYaw` true)))

(event `self.ReceiveBeginPlay`
  (`|ExecutionSequence`
    (:`then_0`
      ;[1 1 1] Spawn and attach gun to player
      (bind _returnvalue (`|SpawnActorFromClass` "/Game/Weapons/BP_WeaponSciFiRifle.BP_WeaponSciFiRifle_C" (`SceneComponent.GetSocketTransform` (`self.Mesh`) "None" "RTS_World") "Undefined" "OverrideRootScale" null null))
      (bind _output_get (set `self.BP_DarknessRifle` _returnvalue))
      (`self.K2_AttachToComponent` _output_get (`self.Mesh`) (`self.SocketName`) "SnapToTarget" "SnapToTarget" "SnapToTarget" true))
    (:`then_1`
      (set `self.Camera Field Of View` (`CameraComponent.FieldOfView` (`self.Camera`))))))

(event `self.ReceiveTick`
  (params (DeltaSeconds :type "Float (single-precision)"))
  (set `self.Delta Seconds` DeltaSeconds))

(event `InputAction|LeaningLeft`
  (params (Key :type "Key Structure"))
  ;[1 1 1] Leaning Update Logic
  (:`Pressed`
    (bind (_direction _leaning_amount) (`Timeline|LeningTimeLineLeft` :!label _label)
      (:`Update`
        (set `self.LeaningAmount` _leaning_amount)
        (`self.SR_Leaning`))))
  (:`Released`
    (goto _label :!via `Reverse`)))

(event `InputAction|ThrowGranade`
  (params (Key :type "Key Structure"))
  ;[1 1 1] GranadeThrowLogic
  (:`Pressed`
    (if (and (not (`self.IsShooting`)) (not (`self.IsAimingGun`)) (> (`self.GranadeAmount`) 0))
      (set `self.CanThrowGrenade` true))))

(event `InputAxis|MoveFoward`
  (params (AxisValue :type "Float (single-precision)"))
  ;[1 1 1] Move Forward & Right
  (`self.FInterpMaxWalkSpeed`)
  (`self.AddMovementInput` (`KismetMathLibrary.GetForwardVector` (`KismetMathLibrary.MakeRotator` 0.0 0.0 (.yaw (`self.GetControlRotation`)))) AxisValue))

(event `InputAxis|TurnRate`
  (params (AxisValue :type "Float (single-precision)"))
  ;[1 1 1] MouseInput
  ;;[1 1 1] Yaw -- Z Axis
  (`self.AddControllerYawInput` (* AxisValue (`self.BaseTurnRate`) (`GameplayStatics.GetWorldDeltaSeconds`))))

(event `SR_Leaning`
  ;[1 1 1] Leaning Update Logic
  (set `self.LeaningAmount` (`self.LeaningAmount`)))

(event `InputAxis|LookUpRate`
  (params (AxisValue :type "Float (single-precision)"))
  ;[1 1 1] MouseInput
  ;;[1 1 1] Pitch -- Y Axis
  (`self.AddControllerPitchInput` (* AxisValue (`self.BaseLookUpRate`) (`GameplayStatics.GetWorldDeltaSeconds`))))

(event `InputAction|Melee`
  (params (Key :type "Key Structure"))
  (:`Pressed`
    (`self.PlayAnimMontage` "/Game/Character/Animation/Actions/AM_Melee.AM_Melee" 2.0)))

(event `InputAction|LeaningRight`
  (params (Key :type "Key Structure"))
  ;[1 1 1] Leaning Update Logic
  (:`Pressed`
    (bind (_direction _leaning_amount) (`Timeline|LeaningTimeLineRight` :!label _label_2)
      (:`Update`
        (set `self.LeaningAmount` _leaning_amount)
        (`self.SR_Leaning`))))
  (:`Released`
    (goto _label_2 :!via `Reverse`)))

(event `InputAction|Sprint`
  (params (Key :type "Key Structure"))
  ;[1 1 1] Set Sprinting
  (:`Pressed`
    (set `self.Sprinting` true)
    (set `self.WalkSpeed` (`KismetMathLibrary.FClamp` (* (`self.WalkSpeed`) 3.0) 600.0 1000.0)))
  (:`Released`
    (set `self.Sprinting` false)
    (set `self.WalkSpeed` (`KismetMathLibrary.FClamp` (* (`self.WalkSpeed`) 3.0) 600.0 600.0))))

(event `InputAction|Walk`
  (params (Key :type "Key Structure"))
  ;[1 1 1] Set Walking
  (:`Pressed`
    (`/Engine/EditorBlueprintResources/StandardMacros.FlipFlop`
      (:`A`
        (`self.SR_Walking`)
        (set `self.Walking` true)
        (set `self.WalkSpeed` (`KismetMathLibrary.FClamp` (* (`self.WalkSpeed`) 3.0) 600.0 300.0)))
      (:`B`
        (`self.SR_Jog`)
        (set `self.Walking` false)
        (set `self.WalkSpeed` (`KismetMathLibrary.FClamp` (* (`self.WalkSpeed`) 3.0) 600.0 600.0))))))

(event `SR_Walking`
  ;[1 1 1] Set Walking
  (set `self.Walking` true)
  (set `self.WalkSpeed` (`KismetMathLibrary.FClamp` (* (`self.WalkSpeed`) 3.0) 600.0 300.0)))

(event `SR_Jog`
  ;[1 1 1] Set Walking
  (set `self.Walking` false)
  (set `self.WalkSpeed` (`KismetMathLibrary.FClamp` (* (`self.WalkSpeed`) 3.0) 600.0 600.0)))

(event `InputAction|TogleInventory`
  (params (Key :type "Key Structure"))
  (bind _inventoryactor (`self.InventoryActor`))
  (bind _charactermovement (`self.CharacterMovement`))
  (bind _inventorywidget (`self.InventoryWidget`))
  ;[1 1 1] Inventory
  (:`Pressed`
    (`/Engine/EditorBlueprintResources/StandardMacros.FlipFlop`
      (:`A`
        (`SceneComponent.SetVisibility` _inventoryactor true false)
        (`/Engine/EditorBlueprintResources/StandardMacros.IsValid` null
          (:`Is Valid`
            (`Widget.SetVisibility` _inventorywidget "Visible")
            (`self.InputModeUI` (`self.InventoryWidget`)))
          (:`Is Not Valid`
            (bind _returnvalue (`|CreateWidget` "/Game/HUD/BP_InventoryWidget.BP_InventoryWidget_C"))
            (bind _output_get (set `self.InventoryWidget` _returnvalue))
            (`self.InputModeUI` _output_get)))
        (set `self.IsInInventory?` true)
        (`self.SR_InventoryTogleON`)
        (set `CharacterMovementComponent.bOrientRotationToMovement` false _charactermovement)
        (bind (_direction _zoomin) (`Timeline|Timeline_2` :!via `PlayFromStart`)
          (:`Update`
            (set `CameraComponent.FieldOfView` (- (`self.Camera Field Of View`) _zoomin) (`self.Camera`)))))
      (:`B`
        (`SceneComponent.SetVisibility` _inventoryactor false false)
        (`Widget.SetVisibility` _inventorywidget "Collapsed")
        (`self.InputModeGame`)
        (set `self.IsInInventory?` false)
        (`self.SR_InvenrotyTogleOF`)
        (set `CharacterMovementComponent.bOrientRotationToMovement` true _charactermovement)
        (bind (_direction_2 _zoomin_2) (`Timeline|Timeline_3` :!via `ReverseFromEnd`)
          (:`Update`
            (set `CameraComponent.FieldOfView` (- (`self.Camera Field Of View`) _zoomin_2) (`self.Camera`))))))))

(event `InputAction|InventoryInteraction`
  (params (Key :type "Key Structure"))
  (bind _widgetinteraction (`self.WidgetInteraction`))
  ;[1 1 1] Inventory
  (:`Pressed`
    (`WidgetInteractionComponent.PressPointerKey` _widgetinteraction "LeftMouseButton"))
  (:`Released`
    (`WidgetInteractionComponent.ReleasePointerKey` _widgetinteraction "LeftMouseButton")))

(event `SR_InventoryTogleON`
  ;[1 1 1] Inventory
  (`SceneComponent.SetVisibility` (`self.InventoryActor`) true false)
  (`Widget.SetVisibility` (`self.InventoryWidget`) "Visible"))

(event `SR_InvenrotyTogleOF`
  ;[1 1 1] Inventory
  (`SceneComponent.SetVisibility` (`self.InventoryActor`) false false)
  (`Widget.SetVisibility` (`self.InventoryWidget`) "Collapsed"))

(event `InputAction|ActionKey`
  (params (Key :type "Key Structure"))
  (bind _laserarrow (`/Game/Weapons/BP_WeaponSciFiRifle.LaserArrow` (`self.BP_DarknessRifle`)))
  (bind _returnvalue (`SceneComponent.K2_GetComponentLocation` _laserarrow))
  ;[1 1 1] InteractionLineTrace
  (:`Pressed`
    (bind (_outhit _returnvalue_2) (`KismetSystemLibrary.LineTraceSingle` :`Start` _returnvalue :`End` (+ _returnvalue (* (`SceneComponent.GetForwardVector` _laserarrow) 200.0)) :`TraceChannel` "TraceTypeQuery1" :`bTraceComplex` true :`DrawDebugType` "ForDuration"))
    (if _returnvalue_2
      (set `self.Hit Actor` (`.HitActor` (`GameplayStatics.BreakHitResult` _outhit)))
      (bind _returnvalue_3 (`GameplayStatics.GetActorOfClass` "/Game/Maps/Structures/Hospital/Elevator/BP_ElevatorCharacter.BP_ElevatorCharacter_C"))
      (bind _output_get (set `self.BP_Elevator` _returnvalue_3))
      (if (`/Game/Maps/Structures/Hospital/Elevator/BP_ElevatorCharacter.IsInElevatorArea` _returnvalue_3)
        (bind _output_get_2 (set `/Game/Maps/Structures/Hospital/Elevator/BP_ElevatorCharacter.OpenDoor` true _output_get))
        (`KismetSystemLibrary.PrintString` (`KismetStringLibrary.Concat_StrStr` "ButtonHIT" (`KismetStringLibrary.Conv_BoolToString` _output_get_2)))
        (`KismetSystemLibrary.Delay` 5.0)
        (set `/Game/Maps/Structures/Hospital/Elevator/BP_ElevatorCharacter.OpenDoor` false (`self.BP_Elevator`))))))

(event `GrabBack`
  (bind _charactermovement (`self.CharacterMovement`))
  ;[1 0 0.05556] If Weapon is equiped change socket and rotation system
  (if (`KismetSystemLibrary.IsValid` (`self.BP_DarknessRifle`))
    (`/Engine/EditorBlueprintResources/StandardMacros.FlipFlop`
      (:`A`
        (`self.K2_AttachToComponent` (`self.BP_DarknessRifle`) (`self.Mesh`) "WeaponHand" "SnapToTarget" "SnapToTarget" "SnapToTarget" true)
        (set `self.EquipWeaponBP` true)
        (set `CharacterMovementComponent.bOrientRotationToMovement` false _charactermovement)
        (set `self.bUseControllerRotationYaw` true))
      (:`B`
        (`self.K2_AttachToComponent` (`self.BP_DarknessRifle`) (`self.Mesh`) "KeeperWeapon" "SnapToTarget" "SnapToTarget" "SnapToTarget" true)
        (set `self.EquipWeaponBP` false)
        (set `CharacterMovementComponent.bOrientRotationToMovement` true _charactermovement)
        (set `self.bUseControllerRotationYaw` false)))))

(event `InputAction|FireWeapon`
  (params (Key :type "Key Structure"))
  (bind _bp_darknessrifle (`self.BP_DarknessRifle`))
  (bind _asbp_anim_swat (cast `/Game/Character/Blueprints/BP_AnimSwat` (`SkeletalMeshComponent.GetAnimInstance` (`self.Mesh`)) :!pure true))
  ;[1 1 1] Shooting Gun
  (:`Pressed`
    (if (not (or (`AnimInstance.Montage_IsPlaying` _asbp_anim_swat "/Game/Character/Animation/BS_RifleAnims/AnimMontage/AnimMontageSwatGrabRifle.AnimMontageSwatGrabRifle") (`self.IsReloading`) (`AnimInstance.Montage_IsPlaying` _asbp_anim_swat "/Game/Character/Animation/BS_RifleAnims/AnimMontage/ReloadAnimMontage.ReloadAnimMontage") (`self.IsInInventory?`)))
      (`|ExecutionSequence`
        (:`then_0`
          (goto _label_3 :!via `Open`))
        (:`then_1`
          (`/Engine/EditorBlueprintResources/StandardMacros.Gate` true :!label _label_3
            (:`Exit`
              (`|ExecutionSequence`
                (:`then_0`
                  (if (not (`self.IsReloading`))
                    (if (not (`AnimInstance.Montage_IsPlaying` (cast `/Game/Character/Blueprints/BP_AnimSwat` (`SkeletalMeshComponent.GetAnimInstance` (`self.Mesh`)) :!pure true) "/Game/Character/Animation/BS_RifleAnims/AnimMontage/AnimMontageSwatGrabRifle.AnimMontageSwatGrabRifle"))
                      (set `self.IsShooting` true)
                      (`/Game/Weapons/BP_Weapons.Fire` _bp_darknessrifle)
                      (`GameplayStatics.PlaySoundAtLocation` "/Game/Sounds/SoundsCues/Rifle/Shooting/SC_RifleShooting.SC_RifleShooting" (`SceneComponent.GetSocketLocation` (`/Game/Weapons/BP_WeaponSciFiRifle.Arrow` _bp_darknessrifle) "Muzzle") (struct) 1.0 1.0 0.0 null null null))))
                (:`then_1`
                  (`KismetSystemLibrary.RetriggerableDelay` 0.1)
                  (goto _label_3))
                (:`then_2`
                  (`self.SR_ShootingGun`)))))))))
  (:`Released`
    (set `self.IsShooting` false)
    (goto _label_3 :!via `Close`)))

(event `SR_ShootingGun`
  (bind _bp_darknessrifle (`self.BP_DarknessRifle`))
  ;[1 1 1] Shooting Gun
  (if (not (`self.IsReloading`))
    (if (not (`AnimInstance.Montage_IsPlaying` (cast `/Game/Character/Blueprints/BP_AnimSwat` (`SkeletalMeshComponent.GetAnimInstance` (`self.Mesh`)) :!pure true) "/Game/Character/Animation/BS_RifleAnims/AnimMontage/AnimMontageSwatGrabRifle.AnimMontageSwatGrabRifle"))
      (set `self.IsShooting` true)
      (`/Game/Weapons/BP_Weapons.Fire` _bp_darknessrifle)
      (`GameplayStatics.PlaySoundAtLocation` "/Game/Sounds/SoundsCues/Rifle/Shooting/SC_RifleShooting.SC_RifleShooting" (`SceneComponent.GetSocketLocation` (`/Game/Weapons/BP_WeaponSciFiRifle.Arrow` _bp_darknessrifle) "Muzzle") (struct) 1.0 1.0 0.0 null null null))))

(event `InputAction|AimGun`
  (params (Key :type "Key Structure"))
  (bind _charactermovement (`self.CharacterMovement`))
  (bind _bp_darknessrifle (`self.BP_DarknessRifle`))
  ;[1 1 1] AimingGun
  (:`Pressed`
    (if (and (not (`self.IsReloading`)) (not (`self.IsInInventory?`)) (> (`/Game/Weapons/BP_Weapons.AmmoCount` (`self.BP_DarknessRifle`)) 0))
      (`self.SR_AimingGun`)
      (`|ExecutionSequence`
        (:`then_0`
          (`/Engine/EditorBlueprintResources/StandardMacros.FlipFlop`
            (:`A`
              (set `CharacterMovementComponent.bOrientRotationToMovement` true _charactermovement)
              (set `self.bUseControllerRotationYaw` true)
              (set `self.IsAimingGun` true))
            (:`B`
              (set `CharacterMovementComponent.bOrientRotationToMovement` true _charactermovement)
              (set `self.bUseControllerRotationYaw` true)
              (set `self.IsAimingGun` false)
              (if (`self.IsInZoom`)
                (bind (_direction _zoomin) (`Timeline|Timeline_1` :!via `ReverseFromEnd`)
                  (:`Update`
                    (set `CameraComponent.FieldOfView` (- (`self.Camera Field Of View`) _zoomin) (`self.Camera`))
                    (set `self.IsInZoom` false)))))))
        (:`then_1`
          (`/Engine/EditorBlueprintResources/StandardMacros.FlipFlop`
            (:`A`
              (`/Game/Weapons/BP_WeaponSciFiRifle.SR_LaserSpawn` _bp_darknessrifle))
            (:`B`
              (`ActorComponent.K2_DestroyComponent` (`/Game/Weapons/BP_WeaponSciFiRifle.LaserParticle` _bp_darknessrifle))
              (`ActorComponent.K2_DestroyComponent` (`/Game/Weapons/BP_WeaponSciFiRifle.LaserEnd` _bp_darknessrifle)))))))))

(event `SR_AimingGun`
  (bind _bp_darknessrifle (`self.BP_DarknessRifle`))
  ;[1 1 1] AimingGun
  (`|ExecutionSequence`
    (:`then_0`
      (`/Engine/EditorBlueprintResources/StandardMacros.FlipFlop`
        (:`A`
          (set `self.IsAimingGun` true))
        (:`B`
          (set `self.IsAimingGun` false))))
    (:`then_1`
      (`/Engine/EditorBlueprintResources/StandardMacros.FlipFlop`
        (:`A`
          (`/Game/Weapons/BP_WeaponSciFiRifle.SR_LaserSpawn` _bp_darknessrifle))
        (:`B`
          (`ActorComponent.K2_DestroyComponent` (`/Game/Weapons/BP_WeaponSciFiRifle.LaserParticle` _bp_darknessrifle))
          (`ActorComponent.K2_DestroyComponent` (`/Game/Weapons/BP_WeaponSciFiRifle.LaserEnd` _bp_darknessrifle)))))))

(event `InputAction|OnOfLanternLaser`
  (params (Key :type "Key Structure"))
  (bind _flashlight (`/Game/Weapons/BP_WeaponSciFiRifle.Flashlight` (`self.BP_DarknessRifle`)))
  ;[1 1 1] Lantern
  (:`Pressed`
    (`self.SR_LanterOn`)
    (`/Engine/EditorBlueprintResources/StandardMacros.FlipFlop`
      (:`A`
        (`SceneComponent.SetVisibility` _flashlight true false))
      (:`B`
        (`self.SR_LanterOff`)
        (`SceneComponent.SetVisibility` _flashlight false false)))))

(event `SR_LanterOn`
  ;[1 1 1] Lantern
  (`SceneComponent.SetVisibility` (`/Game/Weapons/BP_WeaponSciFiRifle.Flashlight` (`self.BP_DarknessRifle`)) true false))

(event `SR_LanterOff`
  ;[1 1 1] Lantern
  (`SceneComponent.SetVisibility` (`/Game/Weapons/BP_WeaponSciFiRifle.Flashlight` (`self.BP_DarknessRifle`)) false false))

(event `InputAction|Jump/Climb/Vault`
  (params (Key :type "Key Structure"))
  (bind (_returnvalue_roll _returnvalue_pitch) (`KismetMathLibrary.BreakRotator` (`self.K2_GetActorRotation`)))
  (bind _vaultarrow (`self.VaultArrow`))
  (bind _returnvalue (`SceneComponent.K2_GetComponentLocation` _vaultarrow))
  (bind _returnvalue_2 (+ (`self.K2_GetActorLocation`) (* (`KismetMathLibrary.GetForwardVector` (`KismetMathLibrary.MakeRotFromX` (`self.Wall Normal`))) 50.0)))
  (bind _returnvalue_3 (+ (+ (`self.Wall Location`) (* (`KismetMathLibrary.GetForwardVector` (`KismetMathLibrary.MakeRotFromX` (`self.Wall Normal`))) -50.0)) (0.0 0.0 10.0)))
  (bind _returnvalue_4 (+ (+ (`self.Wall Location`) (* (`KismetMathLibrary.GetForwardVector` (`KismetMathLibrary.MakeRotFromX` (`self.Wall Normal`))) -10.0)) (0.0 0.0 10.0)))
  ;[1 1 1] Vault&Climbing
  (:`Pressed`
    (bind (_outhit _returnvalue_5) (`KismetSystemLibrary.LineTraceSingleForObjects` :`Start` _returnvalue :`End` (+ _returnvalue (* (`SceneComponent.GetForwardVector` _vaultarrow) 70.0)) :`ObjectTypes` (`|MakeArray` "ObjectTypeQuery1" :!type "EObjectTypeQuery Enum") :`bTraceComplex` true :`DrawDebugType` "ForDuration"))
    (if _returnvalue_5
      (bind (_bblockinghit _binitialoverlap _time _distance _location _impactpoint _normal) (`GameplayStatics.BreakHitResult` _outhit))
      (set `self.Wall Location` _location)
      (set `self.Wall Normal` _normal)
      (bind (_outhit_2 _returnvalue_6) (`KismetSystemLibrary.LineTraceSingleForObjects` :`Start` _returnvalue_4 :`End` (- _returnvalue_4 (0.0 0.0 -200.0)) :`ObjectTypes` (`|MakeArray` "ObjectTypeQuery1" :!type "EObjectTypeQuery Enum") :`bTraceComplex` true :`DrawDebugType` "ForDuration"))
      (if _returnvalue_6
        (set `self.Wall Height` (`.Location` (`GameplayStatics.BreakHitResult` _outhit_2)))
        (`|ExecutionSequence`
          (:`then_0`
            (if (> (.z (- (`self.Wall Location`) (`self.Wall Height`))) 60.0)
              (set `self.ShouldClimb?` true)
              (else
                (set `self.ShouldClimb?` false))))
          (:`then_1`
            (bind (_outhit_3 _returnvalue_7) (`KismetSystemLibrary.LineTraceSingleForObjects` :`Start` _returnvalue_3 :`End` (- _returnvalue_3 (0.0 0.0 -250.0)) :`ObjectTypes` (`|MakeArray` "ObjectTypeQuery1" :!type "EObjectTypeQuery Enum") :`bTraceComplex` true :`DrawDebugType` "ForDuration"))
            (if _returnvalue_7
              (set `self.WallHeight2` (`.Location` (`GameplayStatics.BreakHitResult` _outhit_3)))
              (`|ExecutionSequence`
                (:`then_0`
                  (if (> (.z (- (`self.Wall Height`) (`self.WallHeight2`))) 30.0)
                    (set `self.IsWallThick?` false)
                    (else
                      (set `self.IsWallThick?` true))))
                (:`then_1`
                  (if (not (`self.ShouldClimb?`)) :!label _label_4
                    (`PrimitiveComponent.SetCollisionEnabled` (`self.CapsuleComponent`) "NoCollision")
                    (`CharacterMovementComponent.SetMovementMode` (`self.CharacterMovement`) "MOVE_Flying" 0)
                    (if (`self.IsWallThick?`)
                      (`self.K2_SetActorLocation` _returnvalue_2)
                      (bind _returnvalue_8 (`self.PlayAnimMontage` "/Game/Character/Animation/Parkour/AM_Climbing.AM_Climbing"))
                      (`KismetSystemLibrary.Delay` _returnvalue_8)
                      (else
                        (`self.K2_SetActorLocation` _returnvalue_2)
                        (bind _returnvalue_9 (`self.PlayAnimMontage` "/Game/Character/Animation/Parkour/AM_Vault.AM_Vault"))
                        (`KismetSystemLibrary.Delay` _returnvalue_9)))
                    (`self.K2_SetActorRotation` (`KismetMathLibrary.MakeRotator` _returnvalue_roll _returnvalue_pitch (+ (.yaw (`KismetMathLibrary.MakeRotFromX` (`self.Wall Normal`))) 180.0)))
                    (`PrimitiveComponent.SetCollisionEnabled` (`self.CapsuleComponent`) "QueryAndPhysics")
                    (`CharacterMovementComponent.SetMovementMode` (`self.CharacterMovement`) "MOVE_Walking" 0))))
              (else
                (set `self.IsWallThick?` false)
                (goto _label_4)))))))))

(event `InputAction|Crouch`
  (params (Key :type "Key Structure"))
  (bind _returnvalue (`SkeletalMeshComponent.GetAnimInstance` (`self.Mesh`)))
  ;[1 1 1] Crouching
  (:`Pressed`
    (`/Engine/EditorBlueprintResources/StandardMacros.FlipFlop`
      (:`A`
        (`self.SR_Crounching`)
        (set `self.IsCrouching` true)
        (set `self.WalkSpeed` (`KismetMathLibrary.FClamp` (* (`self.WalkSpeed`) 3.0) 300.0 300.0))
        (`self.Crouch`)
        (`AnimInstance.Montage_Play` _returnvalue "/Game/Character/Animation/Anim_Retarget/Retarget_Stand_to_Crouch_Rifle_Hip_Montage.Retarget_Stand_to_Crouch_Rifle_Hip_Montage" 1.0 "MontageLength" 0.0 true))
      (:`B`
        (`self.SR_NotCrounching`)
        (set `self.IsCrouching` false)
        (set `self.WalkSpeed` (`KismetMathLibrary.FClamp` (* (`self.WalkSpeed`) 3.0) 600.0 600.0))
        (`self.UnCrouch`)
        (`AnimInstance.Montage_Play` _returnvalue "/Game/Character/Animation/Anim_Retarget/Retarget_Crouch_to_Stand_Rifle_Hip_Montage.Retarget_Crouch_to_Stand_Rifle_Hip_Montage" 1.0 "MontageLength" 0.0 true)))))

(event `SR_Crounching`
  ;[1 1 1] Crouching
  (set `self.IsCrouching` true)
  (set `self.WalkSpeed` (`KismetMathLibrary.FClamp` (* (`self.WalkSpeed`) 3.0) 300.0 300.0))
  (`self.Crouch`)
  (`AnimInstance.Montage_Play` (`SkeletalMeshComponent.GetAnimInstance` (`self.Mesh`)) "/Game/Character/Animation/Anim_Retarget/Retarget_Stand_to_Crouch_Rifle_Hip_Montage.Retarget_Stand_to_Crouch_Rifle_Hip_Montage" 1.0 "MontageLength" 0.0 true))

(event `SR_NotCrounching`
  ;[1 1 1] Crouching
  (set `self.IsCrouching` false)
  (set `self.WalkSpeed` (`KismetMathLibrary.FClamp` (* (`self.WalkSpeed`) 3.0) 600.0 600.0))
  (`self.UnCrouch`)
  (`AnimInstance.Montage_Play` (`SkeletalMeshComponent.GetAnimInstance` (`self.Mesh`)) "/Game/Character/Animation/Anim_Retarget/Retarget_Crouch_to_Stand_Rifle_Hip_Montage.Retarget_Crouch_to_Stand_Rifle_Hip_Montage" 1.0 "MontageLength" 0.0 true))

(event `InputAxis|MoveRight`
  (params (AxisValue :type "Float (single-precision)"))
  ;[1 1 1] Move Forward & Right
  (`self.FInterpMaxWalkSpeed`)
  (`self.AddMovementInput` (`KismetMathLibrary.GetRightVector` (`KismetMathLibrary.MakeRotator` 0.0 0.0 (.yaw (`self.GetControlRotation`)))) AxisValue))

(event `InputAction|ManualReload`
  (params (Key :type "Key Structure"))
  ;[1 1 1] Reload wen R key is pressed
  (:`Pressed`
    (if (< (`/Game/Weapons/BP_Weapons.AmmoCount` (`self.BP_DarknessRifle`)) 31)
      (set `self.IsReloading` true))))

(event `InputAction|ZoomAim`
  (params (Key :type "Key Structure"))
  ;[1 1 1] ZoomIn & ZoomOut
  (:`Pressed`
    (if (`self.IsAimingGun`)
      (`/Engine/EditorBlueprintResources/StandardMacros.FlipFlop`
        (:`A`
          (bind (_direction _zoomin) (`Timeline|ZoomIn` :!via `PlayFromStart`)
            (:`Update`
              (set `CameraComponent.FieldOfView` (- (`self.Camera Field Of View`) _zoomin) (`self.Camera`))
              (set `self.IsInZoom` true))))
        (:`B`
          (if (`self.IsInZoom`)
            (bind (_direction_2 _zoomin_2) (`Timeline|Timeline_0` :!via `ReverseFromEnd`)
              (:`Update`
                (set `CameraComponent.FieldOfView` (- (`self.Camera Field Of View`) _zoomin_2) (`self.Camera`))
                (set `self.IsInZoom` false)))))))))

(fn `FInterpMaxWalkSpeed`
  (set `CharacterMovementComponent.MaxWalkSpeed` (`KismetMathLibrary.FInterpTo` (`CharacterMovementComponent.MaxWalkSpeed` (`self.CharacterMovement`)) (`self.WalkSpeed`) (`GameplayStatics.GetWorldDeltaSeconds`) 1.5) (`self.CharacterMovement`)))

(fn `Get Rifle Weapon Socket`
  (params (SocketName :type Name))
  (returns (SocketTransform :type "Transform Structure"))
  (bind _bp_darknessrifle (`self.BP_DarknessRifle`))
  (`/Engine/EditorBlueprintResources/StandardMacros.IsValid` _bp_darknessrifle
    (:`Is Valid`
      (return (`SceneComponent.GetSocketTransform` (`/Game/Weapons/BP_Weapons.SkeletalMesh` _bp_darknessrifle) SocketName "RTS_World")))))

(fn `InputModeGame`
  (bind _returnvalue (`GameplayStatics.GetPlayerController` 0))
  (set `PlayerController.bShowMouseCursor` false _returnvalue)
  (`WidgetBlueprintLibrary.SetInputMode_GameOnly` _returnvalue))

(fn `InputModeUI`
  (params (InWidgetToFocus :type "Widget Object Reference"))
  (bind _returnvalue (`GameplayStatics.GetPlayerController` 0))
  (set `PlayerController.bShowMouseCursor` true _returnvalue)
  (`WidgetBlueprintLibrary.SetInputMode_GameAndUIEx` _returnvalue InWidgetToFocus))

(fn `UserConstructionScript`)